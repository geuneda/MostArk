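; BP_Rock_Cannon is a Sand VFX actor that repeatedly fires physics rocks from its position.
; From BeginPlay it loops on a fixed Delay, each pass spawning a BP_Rock at the root transform.
; Each rock gets a strong random impulse along the cannon's local X axis and a random rotation, with an NS_Rock_Impact_Dust Niagara burst at the launch point.
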(event EventBeginPlay
  (bind _returnvalue (Game|SpawnActorfromClass "/Game/Vefects/Sand_VFX/VFX/Rocks/Blueprints/BP_Rock.BP_Rock_C" (Transformation|GetWorldTransform (Variables|Default|GetDefaultSceneRoot)) "Undefined" 0 0 :!label _label))
  (bind _output_get (Variables|Default|SetRockInstance _returnvalue))
  (Physics|AddImpulse (Variables|/Game/Vefects/Sand_VFX/VFX/Rocks/Blueprints/BP_Rock.BP_Rock_C|GetStaticMesh _output_get) (Math|Transform|TransformDirection (Transformation|GetActorTransform) (Math|Vector|MakeVector (Math|Random|RandomFloatinRange 2.5e+05 3e+05) 0.0 0.0)) "None" false)
  (Transformation|SetRelativeRotation (Variables|/Game/Vefects/Sand_VFX/VFX/Rocks/Blueprints/BP_Rock.BP_Rock_C|GetStaticMesh (Variables|Default|GetRockInstance)) (Math|Conversions|RotationFromXVector (Math|Random|RandomUnitVector)) false false)
  (Niagara|SpawnSystematLocation "/Game/Vefects/Sand_VFX/VFX/Rocks/NS_Rock_Impact_Dust.NS_Rock_Impact_Dust" (.location (Transformation|GetWorldTransform (Variables|Default|GetDefaultSceneRoot))))
  (Utilities|FlowControl|Delay 2.0)
  (goto _label))

(fn ConstructionScript)